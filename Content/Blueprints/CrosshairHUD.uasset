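; HUD class that puts the spacesuit interface and a centered crosshair on the player's screen.
; On BeginPlay it creates the SpacesuitHUD widget, stores it and adds it to the viewport.
; Each DrawHUD call draws the fixed-size crosshair texture at screen center, only while the EnableHUD flag on the fetched instance is set.
; That flag gates only the crosshair, not the widget.
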(event EventDrawHUD
  (params (SizeX :type Integer) (SizeY :type Integer))
  (bind _self self)
  (bind _returnvalue (Class|SpaceGameStateBase|Instance _self))
  (if (Variables|/Script/VoidSpace.SpaceGameStateBase|GetbEnableHUD _returnvalue)
    (Canvas|DrawTexture _self "/Game/Textures/Crosshair.Crosshair" (- (Math|Conversions|ToFloat(Integer) (/ SizeX 2)) 25.0) (- (Math|Conversions|ToFloat(Integer) (/ SizeY 2)) 25.0) 5e+01 5e+01 0.0 0.0 1.0 1.0)))

(event EventBeginPlay
  (bind _returnvalue (UserInterface|CreateWidget "/Game/Blueprints/SpacesuitHUD.SpacesuitHUD_C"))
  (bind _output_get (Variables|Default|SetSpacesuitHUD _returnvalue))
  (UserInterface|Viewport|AddtoViewport _output_get 0))

(fn ConstructionScript)