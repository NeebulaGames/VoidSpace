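; HoleTrigger is a Blueprint that finishes an event when a trigger is entered, once its linked Hole has been closed.
; On BeginPlay it disables overlap events on the Interactable's box and binds to the Hole's closed event and the Interactable's trigger-enter event.
; Closing the hole re-enables overlaps and plays an assistant dialogue through the instance's DialogueManager.
; Entering the trigger then calls FinishEvent on the instance.
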(event Custom|CustomEvent_0
  (Class|SpaceGameStateBase|Instance self)
  (Class|SpaceGameStateBase|FinishEvent (stale EventBeginPlay _returnvalue)) ; TODO: Call directly to Event Manager
)

(event Custom|HoleClosed
  (Variables|/Script/Engine.PrimitiveComponent|SetbGenerateOverlapEvents (Variables|/Script/VoidSpace.InteractableComponent|GetBoxComponent (Variables|Default|GetInteractable)) true)
  (Class|DialogueManager|PlayDialogue (Variables|/Script/VoidSpace.SpaceGameStateBase|GetDialogueManager (stale EventBeginPlay _returnvalue)) "Assistant_016"))

(event EventBeginPlay
  (bind _returnvalue (Class|SpaceGameStateBase|Instance self))
  (EventDispatchers|BindEventtoOnTriggerEnter (Variables|Default|GetInteractable) (delegate Custom|CustomEvent_0))
  (Variables|/Script/Engine.PrimitiveComponent|SetbGenerateOverlapEvents (Variables|/Script/VoidSpace.InteractableComponent|GetBoxComponent (Variables|Default|GetInteractable)) false) ; Replace when SetActive
  (EventDispatchers|BindEventtoOnHoleClosed (Variables|Default|GetHole) (delegate Custom|HoleClosed)))

(fn ConstructionScript)